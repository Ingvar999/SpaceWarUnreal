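; Laser gun that fires repeated damaging beam shots along a supplied direction component while shooting is active.
; A looping timer runs LaserShot, which pauses it when shooting is off; StartShotting sets the direction and unpauses it.
; Each shot plays sound, shows a particle beam for half a second, and uses a multi-object line trace to damage Damageable actors along the beam.
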(event EventBeginPlay
  (Utilities|Time|SetTimerbyFunctionName 0 "LaserShot" (Variables|Default|Getdelay) true))

(event Collision|EventActorBeginOverlap
  (params (OtherActor :type Actor%20Object%20Reference)))

(event EventTick
  (params (DeltaSeconds :type Float%20%28single-precision%29)))

(fn ConstructionScript)

(fn LaserShot
  (bind _distance (Variables|Default|Getdistance))
  (bind _direction_object (Variables|Default|Getdirection_object))
  (bind _laseremit (Variables|Default|GetLaserEmit))
  (bind _returnvalue (Transformation|GetWorldLocation _direction_object))
  (bind _returnvalue_2 (Math|Vector|GetForwardVector _direction_object))
  (bind _returnvalue_3 (* _returnvalue_2 _distance))
  (bind _returnvalue_4 (+ _returnvalue _returnvalue_3))
  (if (Variables|Default|Getshotting)
    (Effects|Components|ParticleSystem|SetTemplate (Variables|Default|GetLaserEmit) "/Game/Blueprints/laser/BeamPS.BeamPS")
    (Transformation|SetWorldLocation (Variables|Default|GetDefaultSceneRoot) _returnvalue false false)
    (Class|ParticleSystemComponent|SetBeamSourcePoint _laseremit 0 _returnvalue)
    (Class|ParticleSystemComponent|SetBeamTargetPoint _laseremit 0 _returnvalue_4)
    (Audio|Components|Audio|Play (Variables|Default|Getsf_laser_Cue) 0.0)
    (Utilities|Time|SetTimerbyFunctionName 0 "HideLaser" 0.5)
    (Rendering|SetVisibility _laseremit true true)
    (bind (_outhits _returnvalue_5) (Class|KismetSystemLibrary|LineTraceMultiforObjects _returnvalue _returnvalue_4 (Utilities|Array|MakeArray "ObjectTypeQuery2" "ObjectTypeQuery1" "ObjectTypeQuery3" "ObjectTypeQuery4") false 0 "None" true))
    (if _returnvalue_5
      (for _array_element _outhits
        (bind _asdamageable (Utilities|Casting|CastToDamageable (.HitActor (Collision|BreakHitResult _array_element))))
        (Default|Damage _asdamageable (Variables|Default|Getdamage))))
    (else
      (Class|KismetSystemLibrary|PauseTimer 0 "LaserShot"))))

(fn HideLaser
  (Rendering|SetVisibility (Variables|Default|GetLaserEmit) false false))

(fn StartShotting
  (params (direction_object :type Widget%20Interaction%20Component%20Object%20Reference))
  (Variables|Default|Setdirection_object direction_object)
  (Variables|Default|Setshotting true)
  (Class|KismetSystemLibrary|UnPauseTimer 0 "LaserShot")
  (return false))

(fn StopShotting
  (Variables|Default|Setshotting false)
  (return true))