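; SpaceSkyBox is an actor that displays a space sky on a static mesh with a configurable material.
; It assigns the material and pushes star brightness, power and scene brightness into the SkyBoxParams Material Parameter Collection.
; The construction script and BeginPlay run identical logic, so settings apply both on construction and when play starts.
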(event EventBeginPlay
  (Rendering|Material|SetMaterial (Variables|Default|GetStaticMesh) 0 (Variables|Default|Getmaterial))
  (Rendering|Material|SetScalarParameterValue "/Game/Blueprints/SkyBoxParams.SkyBoxParams" "StarBrightness" (Variables|Default|GetstarBrightness) :!class /Script/Engine.KismetMaterialLibrary)
  (Rendering|Material|SetScalarParameterValue "/Game/Blueprints/SkyBoxParams.SkyBoxParams" "Power" (Variables|Default|Getpower) :!class /Script/Engine.KismetMaterialLibrary)
  (Rendering|Material|SetScalarParameterValue "/Game/Blueprints/SkyBoxParams.SkyBoxParams" "SceneBrightness" (Variables|Default|GetsceneBrightness) :!class /Script/Engine.KismetMaterialLibrary))

(event Collision|EventActorBeginOverlap
  (params (OtherActor :type Actor%20Object%20Reference)))

(event EventTick
  (params (DeltaSeconds :type Float%20%28single-precision%29)))

(fn ConstructionScript
  (Rendering|Material|SetMaterial (Variables|Default|GetStaticMesh) 0 (Variables|Default|Getmaterial))
  (Rendering|Material|SetScalarParameterValue "/Game/Blueprints/SkyBoxParams.SkyBoxParams" "StarBrightness" (Variables|Default|GetstarBrightness) :!class /Script/Engine.KismetMaterialLibrary)
  (Rendering|Material|SetScalarParameterValue "/Game/Blueprints/SkyBoxParams.SkyBoxParams" "Power" (Variables|Default|Getpower) :!class /Script/Engine.KismetMaterialLibrary)
  (Rendering|Material|SetScalarParameterValue "/Game/Blueprints/SkyBoxParams.SkyBoxParams" "SceneBrightness" (Variables|Default|GetsceneBrightness) :!class /Script/Engine.KismetMaterialLibrary))