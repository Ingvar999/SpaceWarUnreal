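; Asteroid actor Blueprint that prints a debug greeting when clicked; it looks like a test or learning asset.
; MyFunction loops a fixed number of times, nudging the static mesh by a local offset without sweep, then returns the input string with a prefix.
; Nothing in the file calls MyFunction, BeginPlay, overlap and Tick are empty, and the macro graph holds only an unused addition.
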(event EventBeginPlay)

(event Collision|EventActorBeginOverlap
  (params (OtherActor :type Actor%20Object%20Reference)))

(event EventTick
  (params (DeltaSeconds :type Float%20%28single-precision%29)))

(event MouseInput|EventActorOnClicked
  (params (ButtonPressed :type Key%20Structure))
  (Development|PrintString "Hello"))

(fn ConstructionScript)

(fn MyFunction
  (params (input_string :type String))
  (Variables|Default|Seti 10)
  (if (> (Variables|Default|Geti) 0) :!label _label
    (Transformation|AddLocalOffset (Variables|Debug|GetStaticMeshComponent) (Variables|Default|Getstructure) false false)
    (Variables|Default|Seti (- (Variables|Default|Geti) 1))
    (goto _label)
    (else
      (return (Utilities|String|Append "I got " input_string)))))