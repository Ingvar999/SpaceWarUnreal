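; Enemy pawn that spawns with a random LaserGun or Machinegun and becomes active after a short delay.
; When PawnSensing sees the player ship, it fires in timed bursts while Tick turns its mesh toward the player, using the controller's spread and reaction values.
; Damage briefly flashes a material, and death notifies SpacePlayerController and destroys gun and pawn.
; Movement and manual rotation logic is disconnected and never runs.
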(event OnSeePawn(PawnSensing)
  (params (Pawn :type Pawn%20Object%20Reference))
  (if (Variables|Default|Getactive)
    (bind _asspace_ship_pawn (Utilities|Casting|CastToSpaceShipPawn Pawn))
    (Variables|Default|Setplayer _asspace_ship_pawn)
    (Variables|Default|Setseeing true)
    (Variables|Default|Settarget_rotation "0, 0, 0")
    (Default|StartShotting (Variables|Default|Getgun) (Variables|Default|GetGunDirection))
    (Utilities|Time|SetTimerbyFunctionName 0 "StopShotting" 2.0)))

(event EventBeginPlay
  (bind _self self)
  (bind _returnvalue (Game|SpawnActorfromClass (Utilities|Select :Index (Math|Random|RandomInteger 2) :Option%200 "/Game/Blueprints/LaserGun.LaserGun_C" :Option%201 "/Game/Blueprints/Machinegun.Machinegun_C") (Transformation|GetWorldTransform (Variables|Default|GetGunDirection)) "AlwaysSpawn" _self _self))
  (Variables|Default|Setgun_actor _returnvalue)
  (bind _asgun (Utilities|Casting|CastToGun _returnvalue))
  (Variables|Default|Setgun _asgun)
  (Variables|Default|Settarget_rotation (Transformation|GetActorRotation))
  (bind _asspace_player_controller (Utilities|Casting|CastToSpacePlayerController (Game|GetPlayerController 0)))
  (Variables|Default|SetSController _asspace_player_controller)
  (Utilities|Time|SetTimerbyFunctionName 0 "Activate" 3.0))

(event Collision|EventActorBeginOverlap
  (params (OtherActor :type Actor%20Object%20Reference)))

(event EventTick
  (params (DeltaSeconds :type Float%20%28single-precision%29))
  (bind _staticmesh (Variables|Default|GetStaticMesh))
  (bind _scontroller (Variables|Default|GetSController))
  (bind _returnvalue (Transformation|GetWorldTransform _staticmesh))
  (bind _enemy_spread (Variables|/Game/Blueprints/SpacePlayerController.SpacePlayerController_C|Getenemy_spread _scontroller))
  (bind (_location _rotation) (Math|Transform|BreakTransform _returnvalue))
  (bind _returnvalue_2 (* _enemy_spread -1.0))
  (bind _returnvalue_3 (Math|Random|RandomFloatinRange _returnvalue_2 _enemy_spread))
  (Variables|Default|Setdelta DeltaSeconds)
  (if (Variables|Default|Getseeing)
    (Transformation|SetWorldRotation (Variables|Default|GetStaticMesh) (Math|Interpolation|RInterpTo (Transformation|GetWorldRotation (Variables|Default|GetStaticMesh)) (Math|Rotator|CombineRotators (Math|Conversions|RotationFromXVector (- (Transformation|GetWorldLocation (Variables|/Game/Blueprints/SpaceShipPawn.SpaceShipPawn_C|GetStaticMesh (Variables|Default|Getplayer))) (Transformation|GetWorldLocation (Variables|Default|GetStaticMesh)))) (Math|Rotator|MakeRotator 0.0 _returnvalue_3 _returnvalue_3)) (Variables|Default|Getdelta) (Variables|/Game/Blueprints/SpacePlayerController.SpacePlayerController_C|Getenemy_reaction (Variables|Default|GetSController))) false false))
  (Transformation|SetWorldLocationAndRotation (Variables|Default|GetPlane%20mesh) _location _rotation false false))

(fn ConstructionScript
  (|CallParentFunction))

(fn IncreaseHP
  (bind _output_get (Variables|Default|SetHealthPoint (+ (Variables|Default|GetHealthPoint) 1))))

(fn SetNormalMaterial
  (Rendering|Material|SetMaterial (Variables|Default|Gett-65) 0 "/DatasmithContent/Materials/Datasmith_Color.Datasmith_Color"))

(fn StopShotting
  (Default|StopShotting (Variables|Default|Getgun))
  (Variables|Default|Setseeing false))

(fn Activate
  (Variables|Default|Setactive true))

(fn Damage
  (params (value :type Integer))
  (bind _output_get (Variables|Default|SetHealthPoint (- (Variables|Default|GetHealthPoint) value)))
  (if (<= _output_get 0)
    (bind _asspace_player_controller (Utilities|Casting|CastToSpacePlayerController (Game|GetPlayerController 0)))
    (Default|OnEnemyDestroyed _asspace_player_controller)
    (Actor|DestroyActor (Variables|Default|Getgun_actor))
    (Actor|DestroyActor)
    (else
      (Rendering|Material|SetMaterial (Variables|Default|Gett-65) 0 "/Game/Blueprints/materials/DamageMaterial.DamageMaterial")
      (Utilities|Time|SetTimerbyFunctionName 0 "SetNormalMaterial" 0.1)))
  (return true))