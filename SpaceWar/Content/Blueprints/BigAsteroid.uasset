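; BigAsteroid is a damageable asteroid obstacle that hurts the player's spaceship on impact.
; On overlap, it damages a SpaceShipPawn in proportion to the ship's speed, if that speed exceeds a threshold.
; Its Damage function reduces Hp and briefly flashes a damage material, restored by a timer.
; When Hp drops below zero, it reports itself to the SpacePlayerController through OnAsteroidDestroy rather than destroying itself.
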(event EventBeginPlay)

(event Collision|EventActorBeginOverlap
  (params (OtherActor :type Actor%20Object%20Reference))
  (bind _asspace_ship_pawn (Utilities|Casting|CastToSpaceShipPawn OtherActor))
  (if (> (Math|Vector|VectorLength (Variables|/Game/Blueprints/SpaceShipPawn.SpaceShipPawn_C|Getspeed _asspace_ship_pawn)) 15.0)
    (Default|Damage _asspace_ship_pawn (Math|Float|Truncate (* (Math|Vector|VectorLength (Variables|/Game/Blueprints/SpaceShipPawn.SpaceShipPawn_C|Getspeed _asspace_ship_pawn)) (Variables|Default|Getbase_damage))))))

(event EventTick
  (params (DeltaSeconds :type Float%20%28single-precision%29)))

(fn ConstructionScript)

(fn SetNormalMaterial
  (Rendering|Material|SetMaterial (Variables|Debug|GetStaticMeshComponent) 0 "/Game/Blueprints/materials/TwoTone.TwoTone"))

(fn Damage
  (params (value :type Integer))
  (bind _output_get (Variables|Default|Sethp (- (Variables|Default|Gethp) value)))
  (if (>= _output_get 0)
    (Rendering|Material|SetMaterial (Variables|Debug|GetStaticMeshComponent) 0 "/Game/Blueprints/materials/DamageMaterial.DamageMaterial")
    (Utilities|Time|SetTimerbyFunctionName self "SetNormalMaterial" 0.1)
    (else
      (bind _asspace_player_controller (Utilities|Casting|CastToSpacePlayerController (Game|GetPlayerController 0)))
      (Default|OnAsteroidDestroy _asspace_player_controller self)))
  (return true))