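; Bullet projectile actor for a spaceship game that damages what it hits.
; On spawn it caches the player ship's Speed, then each Tick moves without sweep along its forward vector, adding that cached value unscaled by delta time.
; Any overlap destroys it and calls Damage on the other actor if it casts to Damageable.
; A timer started after the ship cast succeeds destroys stray bullets after a few seconds.
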(event EventBeginPlay
  (bind _asspace_ship_pawn (Utilities|Casting|CastToSpaceShipPawn (Game|Player|GetPlayerPawn 0)))
  (Variables|Default|Setinit_speed (Variables|/Game/Blueprints/SpaceShipPawn.SpaceShipPawn_C|Getspeed _asspace_ship_pawn))
  (Utilities|Time|SetTimerbyFunctionName self "SelfDestroy" 4.0))

(event Collision|EventActorBeginOverlap
  (params (OtherActor :type Actor%20Object%20Reference))
  (Actor|DestroyActor)
  (bind _asdamageable (Utilities|Casting|CastToDamageable OtherActor))
  (Default|Damage _asdamageable (Variables|Default|Getdamage)))

(event EventTick
  (params (DeltaSeconds :type Float%20%28single-precision%29))
  (Transformation|AddActorWorldOffset (+ (* (Transformation|GetActorForwardVector) (* DeltaSeconds (Variables|Default|Getspeed))) (Variables|Default|Getinit_speed))))

(event EventDestroyed)

(fn ConstructionScript)

(fn SelfDestroy
  (Actor|DestroyActor))