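; Machinegun Blueprint that fires bullets at a fixed interval while shooting is switched on.
; A looping timer set on BeginPlay calls BulletShot, which spawns a Bullet at DirectionObject's world transform and plays a gunshot sound.
; StartShotting stores the DirectionObject, sets the Shotting flag and unpauses the timer.
; StopShotting only clears the flag, so the timer pauses itself on its next call.
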(event EventBeginPlay
  (Utilities|Time|SetTimerbyFunctionName 0 "BulletShot" (Variables|Default|Getdelay) true))

(event Collision|EventActorBeginOverlap
  (params (OtherActor :type Actor%20Object%20Reference)))

(event EventTick
  (params (DeltaSeconds :type Float%20%28single-precision%29)))

(fn ConstructionScript)

(fn BulletShot
  (if (Variables|Default|Getshotting)
    (Game|SpawnActorfromClass "/Game/Blueprints/Bullet.Bullet_C" (Transformation|GetWorldTransform (Variables|Default|Getdirection_object)) "AlwaysSpawn" 0 0)
    (Audio|Components|Audio|Play (Variables|Default|GetGun_Shot_Cue) 0.0)
    (else
      (Class|KismetSystemLibrary|PauseTimer 0 "BulletShot"))))

(fn StartShotting
  (params (direction_object :type Widget%20Interaction%20Component%20Object%20Reference))
  (Variables|Default|Setdirection_object direction_object)
  (Variables|Default|Setshotting true)
  (Class|KismetSystemLibrary|UnPauseTimer 0 "BulletShot")
  (return false))

(fn StopShotting
  (Variables|Default|Setshotting false)
  (return true))