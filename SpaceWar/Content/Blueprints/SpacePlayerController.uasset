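; Player controller for a space shooter that manages the asteroid field and keeps the ship inside the world.
; BeginPlay fills a spherical area with big asteroids, and a looping timer spawns one whenever the count drops below target.
; OnAsteroidDestroy replaces each destroyed non-small asteroid with eight small ones around its position.
; Tick turns a ship that leaves the world radius back toward the center and resets its velocity inward.
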(event EventBeginPlay
  (for _index (range 1 (Variables|Default|Getasteroids_count))
    (Game|SpawnActorfromClass "/Game/Blueprints/BigAsteroid.BigAsteroid_C" (Math|Transform|MakeTransform (Utilities|GetSphereLocation (Variables|Default|Getarea_radius) (Variables|Default|Getcenter))) "AdjustIfPossibleButDontSpawnIfColliding" 0 0))
  (Utilities|Time|SetTimerbyFunctionName self "AsteroidsRestore" 1.0 true))

(event EventTick
  (params (DeltaSeconds :type Float%20%28single-precision%29))
  (bind _asspace_ship_pawn (Utilities|Casting|CastToSpaceShipPawn (Game|Player|GetPlayerPawn 0)))
  (if (> (Math|Vector|VectorLength (- (Transformation|GetWorldLocation (Variables|/Game/Blueprints/SpaceShipPawn.SpaceShipPawn_C|GetStaticMesh _asspace_ship_pawn)) (Variables|Default|Getcenter))) (Variables|Default|Getworld_radius))
    (Variables|/Game/Blueprints/SpaceShipPawn.SpaceShipPawn_C|Setspeed _asspace_ship_pawn (* (Math|Vector|Normalize (* (- (Transformation|GetWorldLocation (Variables|/Game/Blueprints/SpaceShipPawn.SpaceShipPawn_C|GetStaticMesh _asspace_ship_pawn)) (Variables|Default|Getcenter)) -1.0)) 5e+01))
    (Transformation|SetWorldRotation (Variables|/Game/Blueprints/SpaceShipPawn.SpaceShipPawn_C|GetStaticMesh _asspace_ship_pawn) (Math|Conversions|RotationFromXVector (* (- (Transformation|GetWorldLocation (Variables|/Game/Blueprints/SpaceShipPawn.SpaceShipPawn_C|GetStaticMesh _asspace_ship_pawn)) (Variables|Default|Getcenter)) -1.0)) false false)))

(fn ConstructionScript)

(fn AsteroidsRestore
  (bind _outactors (Actor|GetAllActorsOfClass "/Game/Blueprints/BigAsteroid.BigAsteroid_C"))
  (if (< (Utilities|Array|Length _outactors) (Variables|Default|Getasteroids_count))
    (Game|SpawnActorfromClass "/Game/Blueprints/BigAsteroid.BigAsteroid_C" (Math|Transform|MakeTransform (Utilities|GetSphereLocation (Variables|Default|Getarea_radius) (Variables|Default|Getcenter))) "AdjustIfPossibleButDontSpawnIfColliding" 0 0)))

(fn OnAsteroidDestroy
  (params (asteroid :type Actor%20Object%20Reference))
  (LocalVariables|Setasteroid_position (Transformation|GetActorLocation asteroid))
  (Actor|DestroyActor asteroid)
  (Utilities|Casting|CastToSmallAsteroid asteroid
    (:CastFailed
      (for _index (range 1 8)
        (Game|SpawnActorfromClass "/Game/Blueprints/SmallAsteroid.SmallAsteroid_C" (Math|Transform|MakeTransform (Utilities|GetSphereLocation 7e+02 (LocalVariables|Getasteroid_position))) "AdjustIfPossibleButDontSpawnIfColliding" 0 0)))))