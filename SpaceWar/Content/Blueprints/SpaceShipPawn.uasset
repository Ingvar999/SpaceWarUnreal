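; Player spaceship pawn with six-degree flight, two weapons, a settings menu and widget clicking.
; Tick integrates WASD thrust into a capped, damped velocity, moving the mesh without sweep; turn/look axes and Q/E rotate it, while T65 eases into a cosmetic tilt.
; The mouse wheel switches between a line-trace laser that destroys hit actors behind a timed beam effect and a spawned bullet.
; IncreaseHP copies health to MyGameInstance.
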(event EventBeginPlay
  (Input|EnableInput (Game|GetPlayerController 0))
  (Development|PrintString (Utilities|String|ToString(Vector) (Transformation|GetWorldLocation (Variables|Default|GetStaticMesh)))))

(event Collision|EventActorBeginOverlap
  (params (OtherActor :type Actor%20Object%20Reference)))

(event EventTick
  (params (DeltaSeconds :type Float%20%28single-precision%29))
  (bind _acceleration_delta (Variables|Default|Getacceleration_delta))
  (bind _staticmesh (Variables|Default|GetStaticMesh))
  (bind _staticmesh_2 (Variables|Default|GetStaticMesh))
  (bind _returnvalue (Transformation|GetWorldTransform _staticmesh))
  (bind _returnvalue_2 (* DeltaSeconds _acceleration_delta))
  (bind (_location _rotation) (Math|Transform|BreakTransform _returnvalue))
  (Variables|Default|Setdelta DeltaSeconds)
  (bind _output_get (Variables|Default|Setspeed (+ (select (< (Math|Vector|VectorLength (+ (Variables|Default|Getspeed) (* (Transformation|GetActorForwardVector) (* (Variables|Default|Getx_direction) _returnvalue_2)) (* (Transformation|GetActorRightVector) (* (Variables|Default|Gety_direction) _returnvalue_2)))) (Variables|Default|Getmax_speed)) (+ (Variables|Default|Getspeed) (* (Transformation|GetActorForwardVector) (* (Variables|Default|Getx_direction) _returnvalue_2)) (* (Transformation|GetActorRightVector) (* (Variables|Default|Gety_direction) _returnvalue_2))) (Variables|Default|Getspeed)) (* (* (select (< (Math|Vector|VectorLength (+ (Variables|Default|Getspeed) (* (Transformation|GetActorForwardVector) (* (Variables|Default|Getx_direction) _returnvalue_2)) (* (Transformation|GetActorRightVector) (* (Variables|Default|Gety_direction) _returnvalue_2)))) (Variables|Default|Getmax_speed)) (+ (Variables|Default|Getspeed) (* (Transformation|GetActorForwardVector) (* (Variables|Default|Getx_direction) _returnvalue_2)) (* (Transformation|GetActorRightVector) (* (Variables|Default|Gety_direction) _returnvalue_2))) (Variables|Default|Getspeed)) -1) (* (Variables|Default|Getdelta) (Variables|Default|Getstopping_delta))))))
  (Transformation|AddWorldOffset _staticmesh_2 _output_get false false)
  (Transformation|AddLocalRotation _staticmesh_2 (Math|Rotator|MakeRotator (* (Variables|Default|Getdelta) (Math|Conversions|ToFloat(Integer) (Variables|Default|Getrotate_direction)) (Variables|Default|Getrotate_speed)) 0.0 0.0) false false)
  (bind _output_get_2 (Variables|Default|SetRotation (Math|Interpolation|RInterpTo (Variables|Default|GetRotation) (Variables|Default|Gettarget_rotation) (Variables|Default|Getdelta) 2.0)))
  (Transformation|SetRelativeRotation (Variables|Default|Gett-65) _output_get_2 false false)
  (Transformation|SetWorldLocationAndRotation (Variables|Default|GetPlane%20mesh) _location _rotation false false))

(event Input|AxisEvents|InputAxisTurn
  (params (AxisValue :type Float%20%28single-precision%29))
  (Transformation|AddLocalRotation (Variables|Default|GetStaticMesh) (Math|Rotator|MakeRotator 0.0 0.0 AxisValue) false false))

(event Input|AxisEvents|InputAxisLookUp
  (params (AxisValue :type Float%20%28single-precision%29))
  (Transformation|AddLocalRotation (Variables|Default|GetStaticMesh) (Math|Rotator|MakeRotator 0.0 AxisValue 0.0) false false))

(event Input|KeyboardEvents|F
  (params (Key :type Key%20Structure))
  (bind _widgetinteraction1 (Variables|Default|GetWidgetInteraction1))
  (:Pressed
    (Class|WidgetInteractionComponent|PressPointerKey _widgetinteraction1 "LeftMouseButton"))
  (:Released
    (Class|WidgetInteractionComponent|ReleasePointerKey _widgetinteraction1 "LeftMouseButton")))

(event Input|KeyboardEvents|P
  (params (Key :type Key%20Structure))
  (bind _returnvalue (Game|GetPlayerController 0))
  (:Pressed
    (bind _returnvalue_2 (UserInterface|CreateWidget "/Game/Blueprints/Widgets/Settings.Settings_C" _returnvalue))
    (UserInterface|Viewport|AddtoViewport _returnvalue_2 0)
    (Input|SetInputModeUIOnly _returnvalue _returnvalue_2 "DoNotLock")
    (Variables|/Script/Engine.PlayerController|SetbShowMouseCursor _returnvalue true)))

(event Input|MouseEvents|MouseWheelUp
  (params (Key :type Key%20Structure))
  (:Pressed
    (bind _result (Math|Integer|IncrementInt (Variables|Default|GetgunIndex))
      (:%20%20
        (if (> _result 1)
          (Variables|Default|SetgunIndex 0))))))

(event Input|MouseEvents|MouseWheelDown
  (params (Key :type Key%20Structure))
  (:Pressed
    (bind _result (Math|Integer|DecrementInt (Variables|Default|GetgunIndex))
      (:%20%20
        (if (< _result 0)
          (Variables|Default|SetgunIndex 1))))))

(event Input|KeyboardEvents|W
  (params (Key :type Key%20Structure))
  (:Pressed
    (Variables|Default|Setx_direction (+ (Variables|Default|Getx_direction) 1))
    (Variables|Default|Settarget_rotation (Math|Rotator|MakeRotator (+ (.Roll (Math|Rotator|BreakRotator (Variables|Default|Gettarget_rotation))) 7.0) (.Pitch (Math|Rotator|BreakRotator (Variables|Default|Gettarget_rotation))) (.Yaw (Math|Rotator|BreakRotator (Variables|Default|Gettarget_rotation))))))
  (:Released
    (Variables|Default|Setx_direction (+ (Variables|Default|Getx_direction) -1))
    (Variables|Default|Settarget_rotation (Math|Rotator|MakeRotator (+ (.Roll (Math|Rotator|BreakRotator (Variables|Default|Gettarget_rotation))) -7.0) (.Pitch (Math|Rotator|BreakRotator (Variables|Default|Gettarget_rotation))) (.Yaw (Math|Rotator|BreakRotator (Variables|Default|Gettarget_rotation)))))))

(event Input|KeyboardEvents|S
  (params (Key :type Key%20Structure))
  (:Pressed
    (Variables|Default|Setx_direction (+ (Variables|Default|Getx_direction) -1))
    (Variables|Default|Settarget_rotation (Math|Rotator|MakeRotator (+ (.Roll (Math|Rotator|BreakRotator (Variables|Default|Gettarget_rotation))) -7.0) (.Pitch (Math|Rotator|BreakRotator (Variables|Default|Gettarget_rotation))) (.Yaw (Math|Rotator|BreakRotator (Variables|Default|Gettarget_rotation))))))
  (:Released
    (Variables|Default|Setx_direction (+ (Variables|Default|Getx_direction) 1))
    (Variables|Default|Settarget_rotation (Math|Rotator|MakeRotator (+ (.Roll (Math|Rotator|BreakRotator (Variables|Default|Gettarget_rotation))) 7.0) (.Pitch (Math|Rotator|BreakRotator (Variables|Default|Gettarget_rotation))) (.Yaw (Math|Rotator|BreakRotator (Variables|Default|Gettarget_rotation)))))))

(event Input|KeyboardEvents|D
  (params (Key :type Key%20Structure))
  (:Pressed
    (Variables|Default|Sety_direction (+ (Variables|Default|Gety_direction) 1))
    (Variables|Default|Settarget_rotation (Math|Rotator|MakeRotator (.Roll (Math|Rotator|BreakRotator (Variables|Default|Gettarget_rotation))) (+ (.Pitch (Math|Rotator|BreakRotator (Variables|Default|Gettarget_rotation))) 1e+01) (.Yaw (Math|Rotator|BreakRotator (Variables|Default|Gettarget_rotation))))))
  (:Released
    (Variables|Default|Sety_direction (+ (Variables|Default|Gety_direction) -1))
    (Variables|Default|Settarget_rotation (Math|Rotator|MakeRotator (.Roll (Math|Rotator|BreakRotator (Variables|Default|Gettarget_rotation))) (+ (.Pitch (Math|Rotator|BreakRotator (Variables|Default|Gettarget_rotation))) -1e+01) (.Yaw (Math|Rotator|BreakRotator (Variables|Default|Gettarget_rotation)))))))

(event Input|KeyboardEvents|E
  (params (Key :type Key%20Structure))
  (:Pressed
    (Variables|Default|Setrotate_direction (+ (Variables|Default|Getrotate_direction) 1)))
  (:Released
    (Variables|Default|Setrotate_direction (+ (Variables|Default|Getrotate_direction) -1))))

(event Input|KeyboardEvents|A
  (params (Key :type Key%20Structure))
  (:Pressed
    (Variables|Default|Sety_direction (+ (Variables|Default|Gety_direction) -1))
    (Variables|Default|Settarget_rotation (Math|Rotator|MakeRotator (.Roll (Math|Rotator|BreakRotator (Variables|Default|Gettarget_rotation))) (+ (.Pitch (Math|Rotator|BreakRotator (Variables|Default|Gettarget_rotation))) -1e+01) (.Yaw (Math|Rotator|BreakRotator (Variables|Default|Gettarget_rotation))))))
  (:Released
    (Variables|Default|Sety_direction (+ (Variables|Default|Gety_direction) 1))
    (Variables|Default|Settarget_rotation (Math|Rotator|MakeRotator (.Roll (Math|Rotator|BreakRotator (Variables|Default|Gettarget_rotation))) (+ (.Pitch (Math|Rotator|BreakRotator (Variables|Default|Gettarget_rotation))) 1e+01) (.Yaw (Math|Rotator|BreakRotator (Variables|Default|Gettarget_rotation)))))))

(event Input|KeyboardEvents|Q
  (params (Key :type Key%20Structure))
  (:Pressed
    (Variables|Default|Setrotate_direction (+ (Variables|Default|Getrotate_direction) -1)))
  (:Released
    (Variables|Default|Setrotate_direction (+ (Variables|Default|Getrotate_direction) 1))))

(event Input|MouseEvents|LeftMouseButton
  (params (Key :type Key%20Structure))
  (:Pressed
    (switch int (Variables|Default|GetgunIndex)
      (:0
        (Utilities|LaserShot))
      (:1
        (Game|SpawnActorfromClass "/Game/Blueprints/Bullet.Bullet_C" (Transformation|GetWorldTransform (Variables|Default|GetWidgetInteraction1)) "Undefined" 0 0)
        (Audio|Components|Audio|Play (Variables|Default|GetGun_Shot_Cue) 0.1)))))

(fn ConstructionScript
  (|CallParentFunction))

(fn IncreaseHP
  (bind _output_get (Variables|Default|SetHealthPoint (+ (Variables|Default|GetHealthPoint) 1)))
  (bind _output_get_2 (Variables|Default|SethealthString (Utilities|String|ToString(Integer) _output_get)))
  (Development|PrintString _output_get_2)
  (bind _asmy_game_instance (Utilities|Casting|CastToMyGameInstance (Game|GetGameInstance)))
  (Variables|/Game/Blueprints/MyGameInstance.MyGameInstance_C|SethealthPoint _asmy_game_instance _output_get))